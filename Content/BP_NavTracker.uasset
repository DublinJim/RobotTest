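; BP_NavTracker is a robot pawn that navigates toward the BP_PawnForFlag objective in the level.
; On BeginPlay it adds an audio component and plays the bot cue.
; Every Tick it looks up the objective actor and reissues an AI MoveTo to its current location.
; Success and failure each pass through a DoOnce, printing a status message and playing a 2D sound only the first time.
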(event EventBeginPlay
  (AddComponent|AddAudioComponent false)
  (Audio|Components|Audio|Play (Variables|Default|GetThe_bot_Cue) 0.0))

(event EventTick
  (params (DeltaSeconds :type Float%20%28single-precision%29))
  ;[1 1 1] Moveto the Sarah Conner Cube
  (bind _returnvalue (Actor|GetActorOfClass "/Game/BP_PawnForFlag.BP_PawnForFlag_C"))
  (bind _output_get (Variables|Default|SetDestination (Transformation|GetActorLocation _returnvalue)))
  (AI|AIMoveTo self _output_get 0 5.0 false
    (:OnSuccess
      ;[1 1 1] If Found
      (Utilities|FlowControl|DoOnce false
        (:Completed
          (Development|PrintString "Robot has reached objective" true false "(R=0.000000,G=0.660000,B=1.000000,A=1.000000)" 5.0)
          (Audio|PlaySound2D "/Engine/EditorSounds/Notifications/CompileSuccess.CompileSuccess" 1.0 1.0 0.0 0 0 false))))
    (:OnFail
      ;[1 1 1] If Not
      (Utilities|FlowControl|DoOnce false
        (:Completed
          (Development|PrintString "Robot searching for objective" true false "(R=1.000000,G=0.102654,B=0.152417,A=1.000000)" 5.0)
          (Audio|PlaySound2D "/Engine/EditorSounds/Notifications/CompileFailed.CompileFailed" 1.0 1.0 0.0 0 0 false))))))

(fn ConstructionScript)